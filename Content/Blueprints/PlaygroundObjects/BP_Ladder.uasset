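; BP_Ladder is a climbable playground ladder that tells the ThirdPersonCharacter when it is in range to climb.
; Box and TopBox overlaps set the character's near-ladder flag, ladder reference and travel vector from the ladder's up vector.
; Leaving a box clears the ladder flags and restores walking movement.
; An IsAtTop flag, toggled by TopBox, suppresses the lower Box's handling while at the top.
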(event OnComponentBeginOverlap(Box)
  (params (OverlappedComponent :type Primitive%20Component%20Object%20Reference) (OtherActor :type Actor%20Object%20Reference) (OtherComp :type Primitive%20Component%20Object%20Reference) (OtherBodyIndex :type Integer) (bFromSweep :type Boolean) (SweepResult :type Hit%20Result%20Structure%20%28by%20ref%29))
  (if (not (Variables|Default|GetIsAtTop?))
    (bind _asthird_person_character (Utilities|Casting|CastToThirdPersonCharacter OtherActor))
    (Variables|/Game/ThirdPersonBP/Blueprints/ThirdPersonCharacter.ThirdPersonCharacter_C|SetIsNearLadder? _asthird_person_character true)
    (Variables|/Game/ThirdPersonBP/Blueprints/ThirdPersonCharacter.ThirdPersonCharacter_C|SetTravelVector _asthird_person_character (Math|Vector|GetUpVector (Variables|Default|GetLadder)))
    (Variables|/Game/ThirdPersonBP/Blueprints/ThirdPersonCharacter.ThirdPersonCharacter_C|SetLadder _asthird_person_character self)
    (Development|PrintString "NEAR LADDER")))

(event OnComponentEndOverlap(Box)
  (params (OverlappedComponent :type Primitive%20Component%20Object%20Reference) (OtherActor :type Actor%20Object%20Reference) (OtherComp :type Primitive%20Component%20Object%20Reference) (OtherBodyIndex :type Integer))
  (if (not (Variables|Default|GetIsAtTop?))
    (bind _asthird_person_character (Utilities|Casting|CastToThirdPersonCharacter OtherActor))
    (Variables|/Game/ThirdPersonBP/Blueprints/ThirdPersonCharacter.ThirdPersonCharacter_C|SetIsNearLadder? _asthird_person_character false)
    (Variables|/Game/ThirdPersonBP/Blueprints/ThirdPersonCharacter.ThirdPersonCharacter_C|SetIsOnLadder? _asthird_person_character false)
    (Pawn|Components|CharacterMovement|SetMovementMode (Variables|/Script/Engine.Character|GetCharacterMovement _asthird_person_character) "MOVE_Walking" 0)
    (Variables|/Script/Engine.CharacterMovementComponent|SetbUseControllerDesiredRotation (Variables|/Script/Engine.Character|GetCharacterMovement _asthird_person_character) true)
    (Development|PrintString "AWAY FROM LADDER")))

(event OnComponentBeginOverlap(TopBox)
  (params (OverlappedComponent :type Primitive%20Component%20Object%20Reference) (OtherActor :type Actor%20Object%20Reference) (OtherComp :type Primitive%20Component%20Object%20Reference) (OtherBodyIndex :type Integer) (bFromSweep :type Boolean) (SweepResult :type Hit%20Result%20Structure%20%28by%20ref%29))
  (Variables|Default|SetIsAtTop? true)
  (Development|PrintString "IS AT THE TOP")
  (bind _asthird_person_character (Utilities|Casting|CastToThirdPersonCharacter OtherActor))
  (Variables|/Game/ThirdPersonBP/Blueprints/ThirdPersonCharacter.ThirdPersonCharacter_C|SetIsNearLadder? _asthird_person_character true)
  (Variables|/Game/ThirdPersonBP/Blueprints/ThirdPersonCharacter.ThirdPersonCharacter_C|SetTravelVector _asthird_person_character (Math|Vector|GetUpVector (Variables|Default|GetLadder)))
  (Variables|/Game/ThirdPersonBP/Blueprints/ThirdPersonCharacter.ThirdPersonCharacter_C|SetLadder _asthird_person_character self))

(event OnComponentEndOverlap(TopBox)
  (params (OverlappedComponent :type Primitive%20Component%20Object%20Reference) (OtherActor :type Actor%20Object%20Reference) (OtherComp :type Primitive%20Component%20Object%20Reference) (OtherBodyIndex :type Integer))
  (Variables|Default|SetIsAtTop? false)
  (Development|PrintString "NOT AT THE TOP")
  (bind _asthird_person_character (Utilities|Casting|CastToThirdPersonCharacter OtherActor))
  (Variables|/Game/ThirdPersonBP/Blueprints/ThirdPersonCharacter.ThirdPersonCharacter_C|SetIsNearLadder? _asthird_person_character false)
  (Variables|/Game/ThirdPersonBP/Blueprints/ThirdPersonCharacter.ThirdPersonCharacter_C|SetIsOnLadder? _asthird_person_character false)
  (Pawn|Components|CharacterMovement|SetMovementMode (Variables|/Script/Engine.Character|GetCharacterMovement _asthird_person_character) "MOVE_Walking" 0))

(event EventBeginPlay)

(event Collision|EventActorBeginOverlap
  (params (OtherActor :type Actor%20Object%20Reference)))

(event EventTick
  (params (DeltaSeconds :type Float%20%28single-precision%29)))

(fn ConstructionScript)