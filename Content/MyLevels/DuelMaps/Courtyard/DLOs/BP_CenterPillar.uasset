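; Center pillar level object for the Courtyard duel map that rises, runs a rotating beam event, then sinks back.
; While IsActive, Tick moves it toward a point Distance above its start until within a loose tolerance, then after a short delay attaches two spawned BP_Beam actors and starts RotatingMovement.
; A 30-second Delay sets IsEnding, which stops rotation, destroys the beams and lowers the pillar until it deactivates.
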(event EventBeginPlay
  (|CallParentFunction)
  (bind _output_get (Variables|Default|SetStartLocation (Transformation|GetActorLocation)))
  (Variables|Default|SetTopPosition (Math|Vector|MakeVector (.X (Math|Vector|BreakVector _output_get)) (.Y (Math|Vector|BreakVector _output_get)) (+ (.Z (Math|Vector|BreakVector _output_get)) (Variables|Default|GetDistance)))))

(event Collision|EventActorBeginOverlap
  (params (OtherActor :type Actor%20Object%20Reference))
  (|CallParentFunction OtherActor) ; This node is disabled and will not be called.\nDrag off pins to build functionality.
)

(event EventTick
  (params (DeltaSeconds :type Float%20%28single-precision%29))
  (if (Variables|Default|GetIsActive?)
    (CallFunction|PlayObjectEvent)
    (Utilities|FlowControl|Delay 3e+01)
    (Variables|Default|SetIsEnding? true)))

(event EventPlayObjectEnd
  (bind _returnvalue (Transformation|GetActorLocation))
  (bind _beams (Variables|Default|GetBeams))
  (if (Math|Vector|Equal(Vector) (Transformation|GetActorLocation) (Variables|Default|GetStartLocation) 1.0)
    (Variables|Default|SetIsActive? false)
    (else
      (Utilities|FlowControl|Sequence
        (:then_0
          (Utilities|FlowControl|DoOnce false
            (:Completed
              (Components|Activation|SetActive (Variables|Default|GetRotatingMovement) false false)
              (for _array_element _beams
                (Actor|DestroyActor _array_element))
              (Utilities|Array|Clear _beams))))
        (:then_1
          (Transformation|SetWorldLocation (Variables|Default|GetDefaultSceneRoot) (+ (* (Math|Vector|Normalize (- (Variables|Default|GetStartLocation) _returnvalue)) (* (stale EventTick DeltaSeconds) 1e+02)) _returnvalue) false false))))))

(event EventPlayObjectEvent
  (bind _returnvalue (Transformation|GetActorLocation))
  (bind _spawn1 (Variables|Default|GetSpawn1))
  (bind _spawn2 (Variables|Default|GetSpawn2))
  (if (Variables|Default|GetIsEnding?)
    (CallFunction|PlayObjectEnd)
    (else
      (Utilities|FlowControl|Sequence
        (:then_1
          (if (Math|Vector|Equal(Vector) (Transformation|GetActorLocation) (Variables|Default|GetTopPosition) 6e+02)
            (Utilities|FlowControl|Sequence
              (:then_0
                (Utilities|FlowControl|DoOnce false
                  (:Completed
                    (Utilities|FlowControl|Delay 3.0)
                    (bind _returnvalue_2 (Game|SpawnActorfromClass "/Game/MyLevels/DuelMaps/Courtyard/DLOs/BP_Beam.BP_Beam_C" (Transformation|GetWorldTransform _spawn1) "Undefined" 0 0))
                    (Utilities|Array|Add (Variables|Default|GetBeams) _returnvalue_2)
                    (Transformation|AttachComponentToComponent _returnvalue_2 _spawn1 "None" "KeepWorld" "KeepWorld" "KeepWorld" true)
                    (bind _returnvalue_3 (Game|SpawnActorfromClass "/Game/MyLevels/DuelMaps/Courtyard/DLOs/BP_Beam.BP_Beam_C" (Transformation|GetWorldTransform _spawn2) "Undefined" 0 0))
                    (Utilities|Array|Add (Variables|Default|GetBeams) _returnvalue_3)
                    (Transformation|AttachComponentToComponent _returnvalue_3 _spawn2 "None" "KeepWorld" "KeepWorld" "KeepWorld" true)
                    (Components|Activation|Activate (Variables|Default|GetRotatingMovement) false)))))
            (else
              (Transformation|SetWorldLocation (Variables|Default|GetDefaultSceneRoot) (+ (* (Math|Vector|Normalize (- (Variables|Default|GetTopPosition) _returnvalue)) (* (stale EventTick DeltaSeconds) 1e+02)) _returnvalue) false false))))))))

(fn ConstructionScript
  (|CallParentFunction))