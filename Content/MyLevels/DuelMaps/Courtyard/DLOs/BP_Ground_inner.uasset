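; Inner ground object for the Courtyard duel map that fades a material effect in and back out while active.
; Tick raises BlendWeight toward one until a ten-second delay sets IsEnding, then lowers it and clears IsActive near zero.
; ChangeMaterial writes that weight to the static mesh's BlendWeight and EmissivePower parameters.
; Nothing here sets IsActive true or resets IsEnding.
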(event Custom|ChangeMaterial
  (params (Target :type Mesh%20Component%20Object%20Reference) (ParameterValue :type Float%20%28single-precision%29))
  (Rendering|Material|SetScalarParameterValueonMaterials Target "BlendWeight" ParameterValue)
  (Rendering|Material|SetScalarParameterValueonMaterials Target "EmissivePower" ParameterValue))

(event EventBeginPlay
  (|CallParentFunction))

(event Collision|EventActorBeginOverlap
  (params (OtherActor :type Actor%20Object%20Reference))
  (|CallParentFunction OtherActor) ; This node is disabled and will not be called.\nDrag off pins to build functionality.
)

(event EventTick
  (params (DeltaSeconds :type Float%20%28single-precision%29))
  (if (Variables|Default|GetIsActive?)
    (CallFunction|PlayObjectEvent)
    (Utilities|FlowControl|Delay 1e+01)
    (Variables|Default|SetIsEnding? true)))

(event EventPlayObjectEvent
  (if (Variables|Default|GetIsEnding?)
    (CallFunction|PlayObjectEnd)
    (else
      (Utilities|FlowControl|Sequence
        (:then_0
          (if (< (+ (* (stale EventTick DeltaSeconds) 0.1) (Variables|Default|GetBlendWeight)) 1.0)
            (bind _output_get (Variables|Default|SetBlendWeight (+ (* (stale EventTick DeltaSeconds) 0.1) (Variables|Default|GetBlendWeight))))
            (CallFunction|ChangeMaterial (Variables|Default|GetStaticMesh) _output_get)))))))

(event EventPlayObjectEnd
  (if (> (- (Variables|Default|GetBlendWeight) (* (stale EventTick DeltaSeconds) 0.1)) 0.0)
    (bind _output_get (Variables|Default|SetBlendWeight (- (Variables|Default|GetBlendWeight) (* (stale EventTick DeltaSeconds) 0.1))))
    (else
      (Variables|Default|SetIsActive? false)))
  (CallFunction|ChangeMaterial (Variables|Default|GetStaticMesh) _output_get))

(fn ConstructionScript
  (|CallParentFunction))