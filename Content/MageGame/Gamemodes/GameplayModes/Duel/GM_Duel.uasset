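; GM_Duel is the game mode for a two-team duel, handling player tracking, team assignment, a start countdown and respawns.
; ChoosePlayerStart balances teams on DeathMatchPC, gathers ArenaStart actors by team and returns that team's first spawn.
; BeginPlay counts down each second before setting GameStarted, while EveryoneUpdate sends all player settings to each controller.
; Respawn spawns and possesses a BP_MageBase on authority, choosing the side from PS_Duel.OnTeam1.
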(event Custom|SpawnPlayers
  (params (NewParam :type Player%20Controller%20Object%20Reference)))

(event Custom|EveryoneUpdate
  (bind _allplayercontrollers (Variables|Default|GetAllPlayerControllers))
  (bind _output_get (Variables|Default|SetCurrentPlayers (Utilities|Array|Length (Variables|Default|GetAllPlayerControllers))))
  (if (> _output_get 0)
    (Utilities|Array|Clear (Variables|Default|GetConnectedPlayers))
    (for _array_element _allplayercontrollers
      (bind _asdeath_match_pc (Utilities|Casting|CastToDeathMatchPC _array_element))
      (Utilities|Array|Add (Variables|Default|GetConnectedPlayers) (Variables|/Game/MageGame/Gamemodes/GameplayModes/DeathMatch/DeathMatchPC.DeathMatchPC_C|GetPlayerSettings _asdeath_match_pc)))
    (for _array_element_2 _allplayercontrollers
      (bind _asdeath_match_pc_2 (Utilities|Casting|CastToDeathMatchPC _array_element_2))
      (Default|AddPlayerInfo _asdeath_match_pc_2 (Variables|Default|GetConnectedPlayers)))))

(event Custom|Respawn
  (params (controller :type Player%20Controller%20Object%20Reference))
  (Utilities|IsValid controller
    (:Is%20Valid
      (Networking|SwitchHasAuthority
        (:Authority
          (if (Variables|/Game/MageGame/Gamemodes/GameplayModes/Duel/PS_Duel.PS_Duel_C|GetOnTeam1 (.AsPS%20Duel (Utilities|Casting|CastToPS_Duel (Variables|/Script/Engine.Controller|GetPlayerState controller))))
            (bind _returnvalue (Game|SpawnActorfromClass "/Game/MageGame/MageCharacter/BP_MageBase.BP_MageBase_C" (Transformation|GetActorTransform (Utilities|Array|Get(acopy) (Variables|Default|GetTeam1_SpawnPoints))) "Undefined" 0 0))
            (Pawn|Possess controller _returnvalue)
            (else
              (bind _returnvalue_2 (Game|SpawnActorfromClass "/Game/MageGame/MageCharacter/BP_MageBase.BP_MageBase_C" (Transformation|GetActorTransform (Utilities|Array|Get(acopy) (Variables|Default|GetTeam2_SpawnPoints))) "Undefined" 0 0))
              (Pawn|Possess controller _returnvalue_2))))))))

(event EventBeginPlay
  (CallFunction|SpawnPlayers)
  (Utilities|FlowControl|Delay 1.0 :!label _label)
  (Development|PrintString (Utilities|String|ToString(Integer) (Variables|Default|Getcountdown)))
  (if (== (Variables|Default|Getcountdown) 0)
    (Variables|Default|SetGameStarted true)
    (else
      (Variables|Default|Setcountdown (- (Variables|Default|Getcountdown) 1))
      (goto _label))))

(event EventTick
  (params (DeltaSeconds :type Float%20%28single-precision%29)))

(event EventPostLogin
  (params (NewPlayer :type Player%20Controller%20Object%20Reference))
  (Networking|SwitchHasAuthority
    (:Authority
      (Utilities|Array|Add (Variables|Default|GetAllPlayerControllers) NewPlayer))))

(fn ConstructionScript)

(fn ChoosePlayerStart
  (params (Player :type Controller%20Object%20Reference))
  (bind _asdeath_match_pc (Utilities|Casting|CastToDeathMatchPC Player))
  (if (> (Variables|Default|GetNumOfTeam1) (Variables|Default|GetNumOfTeam2))
    (Math|Integer|IncrementInt (Variables|Default|GetNumOfTeam2)
      (:%20%20
        (Variables|/Game/MageGame/Gamemodes/GameplayModes/DeathMatch/DeathMatchPC.DeathMatchPC_C|SetTeam _asdeath_match_pc 1)))
    (else
      (Math|Integer|IncrementInt (Variables|Default|GetNumOfTeam1)
        (:%20%20
          (Variables|/Game/MageGame/Gamemodes/GameplayModes/DeathMatch/DeathMatchPC.DeathMatchPC_C|SetTeam _asdeath_match_pc 0)))))
  (Default|InitialSetup _asdeath_match_pc 1)
  (bind _outactors (Actor|GetAllActorsOfClass "/Game/MageGame/GameObjects/ArenaStart.ArenaStart_C"))
  (bind _array_element (Utilities|Array|ForEachLoopwithBreak _outactors)
    (:LoopBody
      (if (== (Variables|/Game/MageGame/GameObjects/ArenaStart.ArenaStart_C|GetTeam _array_element) 0)
        (Utilities|Array|Add (Variables|Default|GetTeam1_SpawnPoints) _array_element)
        (else
          (Utilities|Array|Add (Variables|Default|GetTeam2_SpawnPoints) _array_element))))
    (:Completed
      (if (== (Variables|/Game/MageGame/Gamemodes/GameplayModes/DeathMatch/DeathMatchPC.DeathMatchPC_C|GetTeam _asdeath_match_pc) 0)
        (return (Utilities|Array|Get(acopy) (Variables|Default|GetTeam1_SpawnPoints)))
        (else
          (return (Utilities|Array|Get(acopy) (Variables|Default|GetTeam2_SpawnPoints))))))))