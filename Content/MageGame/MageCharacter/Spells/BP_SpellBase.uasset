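; BP_SpellBase is a chargeable spell actor for the mage game that explodes on contact.
; Charge grows scale and damage by lerping on each call, flagging overload once CastTime is reached.
; Sphere hits on non-owners destroy it with effects; overlaps with non-instigators also explode, but only BP_MageBase targets take damage and destroy it.
; The BP_SpellShield branch is disconnected, and DecrementHoldTime only prints HoldTime.
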(event OnComponentBeginOverlap(Sphere)
  (params (OverlappedComponent :type Primitive%20Component%20Object%20Reference) (OtherActor :type Actor%20Object%20Reference) (OtherComp :type Primitive%20Component%20Object%20Reference) (OtherBodyIndex :type Integer) (bFromSweep :type Boolean) (SweepResult :type Hit%20Result%20Structure%20%28by%20ref%29))
  (bind (_bblockinghit _binitialoverlap _time _distance _location _impactpoint _normal _impactnormal _physmat _hitactor) (Collision|BreakHitResult SweepResult))
  (if (not (== OtherActor (Game|GetInstigator)))
    (Effects|SpawnEmitteratLocation "/Game/StarterContent/Particles/P_Explosion.P_Explosion" _impactpoint (.rotation (Transformation|GetActorTransform _hitactor)))
    (Audio|PlaySoundatLocation "/Game/StarterContent/Audio/Explosion_Cue.Explosion_Cue" _impactpoint "0, 0, 0" 1.0 1.0 0.0 0 0 0)
    (bind _asbp_mage_base (Utilities|Casting|CastToBP_MageBase _hitactor))
    (Default|TakeDamage _asbp_mage_base (Variables|Damage|GetDamage_Current) (Game|GetInstigator))
    (Actor|DestroyActor)
    (Development|PrintString "spell destroyed by overlap")))

(event OnComponentHit(Sphere)
  (params (HitComponent :type Primitive%20Component%20Object%20Reference) (OtherActor :type Actor%20Object%20Reference) (OtherComp :type Primitive%20Component%20Object%20Reference) (NormalImpulse :type Vector :default "0, 0, 0") (Hit :type Hit%20Result%20Structure%20%28by%20ref%29))
  (bind (_bblockinghit _binitialoverlap _time _distance _location _impactpoint _normal _impactnormal _physmat _hitactor) (Collision|BreakHitResult Hit))
  (if (not (== _hitactor (Components|GetOwner)))
    (Effects|SpawnEmitteratLocation "/Game/StarterContent/Particles/P_Explosion.P_Explosion" _impactpoint (.rotation (Transformation|GetActorTransform _hitactor)))
    (Audio|PlaySoundatLocation "/Game/StarterContent/Audio/Explosion_Cue.Explosion_Cue" _impactpoint "0, 0, 0" 1.0 1.0 0.0 0 0 0)
    (Actor|DestroyActor)
    (Development|PrintString (Utilities|String|Append "Spell Destroyed by " (Utilities|GetDisplayName OtherActor)))))

(event EventBeginPlay)

(event Collision|EventActorBeginOverlap
  (params (OtherActor :type Actor%20Object%20Reference)))

(event EventTick
  (params (DeltaSeconds :type Float%20%28single-precision%29)))

(fn ConstructionScript
  (Transformation|SetActorScale3D (* (Transformation|GetActorScale3D) (Variables|Default|GetBaseSpellSize))))

(fn SetSpellOwner
  (params (Caster :type Actor%20Object%20Reference))
  (Variables|Default|SetSpellOwner Caster))

(fn Charge
  (params (ChargeTime :type Float%20%28single-precision%29))
  (bind _damage_max (Variables|Damage|GetDamage_Max))
  (if (Variables|Default|GetIsOverloaded?)
    (Variables|Default|SetIsOverloaded? true :!label _label)
    (return (Variables|Default|GetIsOverloaded?))
    (else
      (bind _output_get (Variables|Default|SetCurrentCastTime ChargeTime))
      (if (< _output_get (Variables|Default|GetCastTime))
        (if (> (Variables|Default|GetCurrentCastTime) 0.0)
          (Transformation|SetActorScale3D (Math|Vector|Lerp(Vector) (Transformation|GetActorScale3D) (Math|Conversions|ToVector(Float) (+ (Variables|Default|GetCurrentCastTime) (Variables|Default|GetBaseSpellSize))) 0.1))
          (Development|PrintString (Utilities|String|ToString(Float) (Math|Float|Lerp (Variables|Damage|GetDamage_Current) _damage_max 0.1)) true true "(R=1.000000,G=0.112770,B=0.000000,A=1.000000)")
          (Variables|Damage|SetDamage_Current (Math|Float|Clamp(Float) (Math|Float|Lerp (Variables|Damage|GetDamage_Current) _damage_max 0.1) (Variables|Damage|GetDamage_Base) _damage_max))
          (Variables|Default|SetIsOverloaded? false)
          (return (Variables|Default|GetIsOverloaded?)))
        (else
          (goto _label))))))

(fn DecrementHoldTime
  (Development|PrintString (Utilities|String|ToString(Float) (Variables|Default|GetHoldTime)) true true "(R=1.000000,G=0.000000,B=0.000000,A=1.000000)" 58.0))