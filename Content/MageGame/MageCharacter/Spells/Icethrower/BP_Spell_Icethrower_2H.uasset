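; Two-handed icethrower spell actor that sprays an attached ice particle stream and fires projectiles along the mage's camera aim.
; Fire opens a Tick gate, which spawns the emitter once via Release and traces from the first-person camera.
; A 0.1-second Delay paces BP_Flame_Projectile spawns from the two-hand spawn location toward the hit or max range, re-aiming the emitter each shot.
; StopFire deactivates the emitter and closes the gate.
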(event Custom|Fire
  (params (SpawnPoint :type Scene%20Component%20Object%20Reference))
  (bind _spellowner (Variables|Default|GetSpellOwner))
  (bind _asbp_mage_base (Utilities|Casting|CastToBP_MageBase _spellowner))
  (bind _fpcamlocation (Variables|/Game/MageGame/MageCharacter/BP_MageBase.BP_MageBase_C|GetFPCamLocation _asbp_mage_base))
  (bind _fpcamforward (Variables|/Game/MageGame/MageCharacter/BP_MageBase.BP_MageBase_C|GetFPCamForward _asbp_mage_base))
  (bind _returnvalue (* _fpcamforward 1e+03))
  (bind _returnvalue_2 (+ _fpcamlocation _returnvalue))
  (Variables|Default|SetAttachedComponent SpawnPoint)
  (Utilities|FlowControl|Gate true) ; enters at Open
)

(event Custom|Release
  (Utilities|FlowControl|DoOnce false
    (:Completed
      (bind _returnvalue (Effects|SpawnEmitterAttached "/Game/Effects/ConeOfCold/P_IceThrower_2H.P_IceThrower_2H" (Variables|Default|GetAttachedComponent) "None"))
      (Variables|Default|SetParticleSystem _returnvalue))))

(event Custom|StopFire
  (bind _spellowner (Variables|Default|GetSpellOwner))
  (bind _particlesystem (Variables|Default|GetParticleSystem))
  (bind _asbp_mage_base (Utilities|Casting|CastToBP_MageBase _spellowner))
  (bind _fpcamlocation (Variables|/Game/MageGame/MageCharacter/BP_MageBase.BP_MageBase_C|GetFPCamLocation _asbp_mage_base))
  (bind _fpcamforward (Variables|/Game/MageGame/MageCharacter/BP_MageBase.BP_MageBase_C|GetFPCamForward _asbp_mage_base))
  (bind _returnvalue (* _fpcamforward 1e+03))
  (bind _returnvalue_2 (+ _fpcamlocation _returnvalue))
  (CallFunction|Release)
  (Utilities|IsValid _particlesystem
    (:Is%20Valid
      (Components|Activation|Deactivate _particlesystem)
      (Utilities|FlowControl|Gate true) ; enters at Close
    )))

(event Custom|UpdateIce
  (params (NewParam :type Transform))
  (Transformation|SetWorldTransform (Variables|Default|GetParticleSystem) NewParam false false))

(event EventBeginPlay
  (|CallParentFunction) ; This node is disabled and will not be called.\nDrag off pins to build functionality.
)

(event Collision|EventActorBeginOverlap
  (params (OtherActor :type Actor%20Object%20Reference))
  (|CallParentFunction OtherActor) ; This node is disabled and will not be called.\nDrag off pins to build functionality.
)

(event EventTick
  (params (DeltaSeconds :type Float%20%28single-precision%29))
  (bind _spellowner (Variables|Default|GetSpellOwner))
  (bind _asbp_mage_base (Utilities|Casting|CastToBP_MageBase _spellowner))
  (bind _fpcamlocation (Variables|/Game/MageGame/MageCharacter/BP_MageBase.BP_MageBase_C|GetFPCamLocation _asbp_mage_base))
  (bind _fpcamforward (Variables|/Game/MageGame/MageCharacter/BP_MageBase.BP_MageBase_C|GetFPCamForward _asbp_mage_base))
  (bind _returnvalue (* _fpcamforward 1e+03))
  (bind _returnvalue_2 (+ _fpcamlocation _returnvalue))
  (|CallParentFunction DeltaSeconds)
  (Utilities|FlowControl|Sequence
    (:then_1
      (Utilities|FlowControl|Gate true
        (:Exit
          (bind (_outhit _returnvalue_3) (Collision|LineTraceByChannel _fpcamlocation _returnvalue_2 "TraceTypeQuery1" false (Utilities|Array|MakeArray self _spellowner) "None"))
          (Variables|Default|SetStartLocation (Variables|/Game/MageGame/MageCharacter/BP_MageBase.BP_MageBase_C|Get2HSpawnLocation _asbp_mage_base))
          (Utilities|FlowControl|Sequence
            (:then_0
              (CallFunction|Release))
            (:then_1
              (Utilities|FlowControl|Delay 0.1)
              (if _returnvalue_3
                (Variables|Default|SetShootTo (Math|Transform|MakeTransform (Variables|Default|GetStartLocation) (Math|Rotator|FindLookatRotation (Variables|Default|GetStartLocation) (.ImpactPoint (Collision|BreakHitResult _outhit)))))
                (else
                  (Variables|Default|SetShootTo (Math|Transform|MakeTransform (Variables|Default|GetStartLocation) (Math|Rotator|FindLookatRotation (Variables|Default|GetStartLocation) _returnvalue_2)))))
              (bind _returnvalue_4 (Game|SpawnActorfromClass "/Game/MageGame/MageCharacter/Spells/FlameThrower/BP_Flame_Projectile.BP_Flame_Projectile_C" (Variables|Default|GetShootTo) "Undefined" 0 (Variables|Default|GetSpellOwner) 0))
              (Variables|Default|SetProjectileRef _returnvalue_4)
              (CallFunction|UpdateIce (Variables|Default|GetShootTo))
              (for _array_element (Variables|Default|GetIgnoredComponents)
                (Collision|IgnoreActorwhenMoving _array_element 0 true)))))))))

(fn ConstructionScript
  (|CallParentFunction))