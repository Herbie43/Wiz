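; One-handed Icethrower spell that sprays an ice particle stream from the caster's hand while firing.
; Fire opens a Tick gate that traces from the first-person camera and attaches the emitter once; StopFire closes it and deactivates the emitter.
; A 0.1-second Delay throttles spawning of projectiles aimed from the hand at the trace hit or range limit, realigning the emitter with each shot.
; The projectiles reuse BP_Flame_Projectile rather than an ice-specific class.
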(event Custom|Fire
  (params (SpawnPoint :type Scene%20Component%20Object%20Reference) (IsRightHand? :type Boolean))
  (bind _spellowner (Variables|Default|GetSpellOwner))
  (bind _startlocation (Variables|Default|GetStartLocation))
  (bind _asbp_mage_base (Utilities|Casting|CastToBP_MageBase _spellowner))
  (bind _fpcamlocation (Variables|/Game/MageGame/MageCharacter/BP_MageBase.BP_MageBase_C|GetFPCamLocation _asbp_mage_base))
  (bind _fpcamforward (Variables|/Game/MageGame/MageCharacter/BP_MageBase.BP_MageBase_C|GetFPCamForward _asbp_mage_base))
  (bind _returnvalue (* _fpcamforward 1e+03))
  (bind _returnvalue_2 (+ _fpcamlocation _returnvalue))
  (Variables|Default|SetIsRightHand? IsRightHand?)
  (Variables|Default|SetAttachedComponent SpawnPoint)
  (Utilities|FlowControl|Gate true) ; enters at Open
)

(event Custom|Release
  (Utilities|FlowControl|DoOnce false
    (:Completed
      (bind _returnvalue (Effects|SpawnEmitterAttached "/Game/Effects/ConeOfCold/P_IceThrower_1H.P_IceThrower_1H" (Variables|Default|GetAttachedComponent) "None"))
      (Variables|Default|SetParticleSystem _returnvalue))))

(event Custom|StopFire
  (bind _spellowner (Variables|Default|GetSpellOwner))
  (bind _startlocation (Variables|Default|GetStartLocation))
  (bind _asbp_mage_base (Utilities|Casting|CastToBP_MageBase _spellowner))
  (bind _fpcamlocation (Variables|/Game/MageGame/MageCharacter/BP_MageBase.BP_MageBase_C|GetFPCamLocation _asbp_mage_base))
  (bind _fpcamforward (Variables|/Game/MageGame/MageCharacter/BP_MageBase.BP_MageBase_C|GetFPCamForward _asbp_mage_base))
  (bind _returnvalue (* _fpcamforward 1e+03))
  (bind _returnvalue_2 (+ _fpcamlocation _returnvalue))
  (CallFunction|Release)
  (Components|Activation|Deactivate (Variables|Default|GetParticleSystem))
  (Utilities|FlowControl|Gate true) ; enters at Close
)

(event Custom|UpdateIce
  (params (NewParam :type Transform))
  (Transformation|SetWorldTransform (Variables|Default|GetParticleSystem) NewParam false false))

(event EventBeginPlay
  (|CallParentFunction) ; This node is disabled and will not be called.\nDrag off pins to build functionality.
)

(event Collision|EventActorBeginOverlap
  (params (OtherActor :type Actor%20Object%20Reference))
  (|CallParentFunction OtherActor) ; This node is disabled and will not be called.\nDrag off pins to build functionality.
)

(event EventTick
  (params (DeltaSeconds :type Float%20%28single-precision%29))
  (bind _spellowner (Variables|Default|GetSpellOwner))
  (bind _startlocation (Variables|Default|GetStartLocation))
  (bind _asbp_mage_base (Utilities|Casting|CastToBP_MageBase _spellowner))
  (bind _fpcamlocation (Variables|/Game/MageGame/MageCharacter/BP_MageBase.BP_MageBase_C|GetFPCamLocation _asbp_mage_base))
  (bind _fpcamforward (Variables|/Game/MageGame/MageCharacter/BP_MageBase.BP_MageBase_C|GetFPCamForward _asbp_mage_base))
  (bind _returnvalue (* _fpcamforward 1e+03))
  (bind _returnvalue_2 (+ _fpcamlocation _returnvalue))
  (|CallParentFunction DeltaSeconds)
  (Utilities|FlowControl|Sequence
    (:then_1
      (Utilities|FlowControl|Gate true
        (:Exit
          (bind (_outhit _returnvalue_3) (Collision|LineTraceByChannel _fpcamlocation _returnvalue_2 "TraceTypeQuery1" false (Utilities|Array|MakeArray _spellowner self) "None" true "(R=0.000000,G=0.885304,B=1.000000,A=1.000000)"))
          (CallFunction|UpdateSpawnLocation (Variables|Default|GetIsRightHand?))
          (Utilities|FlowControl|Sequence
            (:then_0
              (CallFunction|Release))
            (:then_1
              (Utilities|FlowControl|Delay 0.1)
              (if _returnvalue_3
                (Variables|Default|SetShootTo (Math|Transform|MakeTransform _startlocation (Math|Rotator|FindLookatRotation _startlocation (.ImpactPoint (Collision|BreakHitResult _outhit)))))
                (else
                  (Variables|Default|SetShootTo (Math|Transform|MakeTransform _startlocation (Math|Rotator|FindLookatRotation _startlocation _returnvalue_2)))))
              (bind _returnvalue_4 (Game|SpawnActorfromClass "/Game/MageGame/MageCharacter/Spells/FlameThrower/BP_Flame_Projectile.BP_Flame_Projectile_C" (Variables|Default|GetShootTo) "Undefined" 0 (Variables|Default|GetSpellOwner) 0))
              (Variables|Default|SetProjectileRef _returnvalue_4)
              (CallFunction|UpdateIce (Variables|Default|GetShootTo))
              ;[1 1 1] Shouldn't be necessary with proper collision channels
              (for _array_element (Variables|Default|GetIgnoredComponents)
                (Collision|IgnoreActorwhenMoving _array_element _returnvalue_4 true)))))))))

(fn ConstructionScript
  (|CallParentFunction))

(fn UpdateSpawnLocation
  (params (IsRightHand? :type Boolean))
  (bind _spellowner (Variables|Default|GetSpellOwner))
  (bind _asbp_mage_base (Utilities|Casting|CastToBP_MageBase _spellowner))
  (if IsRightHand?
    (Variables|Default|SetStartLocation (Variables|/Game/MageGame/MageCharacter/BP_MageBase.BP_MageBase_C|GetRHSpawnLocation _asbp_mage_base))
    (else
      (Variables|Default|SetStartLocation (Variables|/Game/MageGame/MageCharacter/BP_MageBase.BP_MageBase_C|GetLHSpawnLocation _asbp_mage_base)))))