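; BP_Spell_Respawn is a channelled utility spell for mages that times a respawn cast; the respawn itself is not handled here.
; Fire or Cast activates SpellEffect at the mage's feet and, first time only, adds a SummonProgress widget and opens a Tick gate.
; While open, the gate accumulates cast time until CastCompleted is set.
; Stopping deactivates the effect, removes the widget, closes the gate and, once only, zeroes CastTime rather than CurrentCastTime.
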(event Custom|Cast
  (params (SpawnPoint :type Scene%20Component%20Object%20Reference))
  (bind _asbp_mage_base (Utilities|Casting|CastToBP_MageBase (Variables|Default|GetSpellOwner)))
  (CallFunction|Activate (Transformation|GetWorldTransform (Variables|/Game/MageGame/MageCharacter/BP_MageBase.BP_MageBase_C|GetFeet_SpawnLocation _asbp_mage_base)))
  (Utilities|FlowControl|DoOnce false
    (:Completed
      (CallFunction|AddSpellUI)
      (Utilities|FlowControl|Gate true) ; enters at Open
    )))

(event Custom|StopCast
  (bind _spelleffect (Variables|Default|GetSpellEffect))
  (CallFunction|Release)
  (Utilities|IsValid _spelleffect
    (:Is%20Valid
      (Components|Activation|Deactivate _spelleffect)
      (CallFunction|RemoveSpellUI)
      (Utilities|FlowControl|Gate true) ; enters at Close
    )))

(event Custom|Release
  (Utilities|FlowControl|DoOnce false
    (:Completed
      (Variables|Default|SetCastTime 0.0)
      (Components|Activation|Deactivate (Variables|Default|GetSpellEffect)))))

(event Custom|Fire
  (params (NewParam :type Scene%20Component%20Object%20Reference))
  (bind _asbp_mage_base (Utilities|Casting|CastToBP_MageBase (Variables|Default|GetSpellOwner)))
  (CallFunction|Activate (Transformation|GetWorldTransform (Variables|/Game/MageGame/MageCharacter/BP_MageBase.BP_MageBase_C|GetFeet_SpawnLocation _asbp_mage_base)))
  (Utilities|FlowControl|DoOnce false
    (:Completed
      (CallFunction|AddSpellUI)
      (Utilities|FlowControl|Gate true) ; enters at Open
    )))

(event Custom|StopFire
  (bind _spelleffect (Variables|Default|GetSpellEffect))
  (CallFunction|Release)
  (Utilities|IsValid _spelleffect
    (:Is%20Valid
      (Components|Activation|Deactivate _spelleffect)
      (CallFunction|RemoveSpellUI)
      (Utilities|FlowControl|Gate true) ; enters at Close
    )))

(event Custom|Activate
  (params (NewParam :type Transform))
  (bind _spelleffect (Variables|Default|GetSpellEffect))
  (Transformation|SetWorldTransform _spelleffect NewParam false false)
  (Components|Activation|Activate _spelleffect false))

(event Custom|AddSpellUI
  (bind _returnvalue (UserInterface|CreateWidget "/Game/MageGame/MageCharacter/Spells/Utility/Respawn/SummonProgress.SummonProgress_C" (.AsPlayer%20Controller (Utilities|Casting|CastToPlayerController (Pawn|GetController (Variables|/Script/Engine.Actor|GetInstigator (Variables|Default|GetSpellOwner))))) self))
  (bind _output_get (Variables|Default|SetSpellUI _returnvalue))
  (UserInterface|Viewport|AddtoViewport _output_get 0)
  (Development|PrintString "Summoning bar added"))

(event Custom|RemoveSpellUI
  (bind _spellui (Variables|Default|GetSpellUI))
  (Utilities|IsValid _spellui
    (:Is%20Valid
      (Widget|RemovefromParent _spellui))))

(event EventBeginPlay
  (|CallParentFunction) ; This node is disabled and will not be called.\nDrag off pins to build functionality.
)

(event Collision|EventActorBeginOverlap
  (params (OtherActor :type Actor%20Object%20Reference))
  (|CallParentFunction OtherActor) ; This node is disabled and will not be called.\nDrag off pins to build functionality.
)

(event EventTick
  (params (DeltaSeconds :type Float%20%28single-precision%29))
  (|CallParentFunction DeltaSeconds)
  (Utilities|FlowControl|Sequence
    (:then_1
      (Utilities|FlowControl|Gate true
        (:Exit
          (if (>= (Variables|Default|GetCurrentCastTime) (Variables|Default|GetCastTime))
            (Variables|Default|SetCastCompleted true)
            (else
              (Variables|Default|SetCurrentCastTime (+ (Variables|Default|GetCurrentCastTime) DeltaSeconds)))))))))

(fn ConstructionScript
  (|CallParentFunction))