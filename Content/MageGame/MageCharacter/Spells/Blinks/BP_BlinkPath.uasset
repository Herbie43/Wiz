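; BP_BlinkPath is a blink spell actor, owned by a mage, that holds a timed path built from BP_BlinkPathSection actors.
; Construction derives the maximum section count from path length and section length.
; AddSection spawns a section at a given location, passing on the duration, and records it in PathSections, without checking that maximum.
; On BeginPlay, a server lifespan event waits out the duration, then destroys the path actor.
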(event Custom|HandleLifespan_OnServer
  (Utilities|FlowControl|Delay (Variables|Default|GetDuration))
  (Utilities|Casting|CastToBP_MageBase (Components|GetOwner))
  (Actor|DestroyActor))

(event Custom|AddSection
  (params (Location :type Vector))
  (bind _returnvalue (Game|SpawnActorfromClass "/Game/MageGame/MageCharacter/Spells/Blinks/BP_BlinkPathSection.BP_BlinkPathSection_C" (Math|Transform|MakeTransform Location "0, 0, 0" "1,1,1") "Undefined" self (Variables|Default|GetDuration) 0))
  (Utilities|Array|Add (Variables|Default|GetPathSections) _returnvalue))

(event EventBeginPlay
  (Utilities|Casting|CastToBP_MageBase (Components|GetOwner))
  (CallFunction|HandleLifespanonServer))

(fn ConstructionScript
  (CallFunction|SetSectionLimit (Variables|Default|GetPathLength)))

(fn SetSectionLimit
  (params (Length :type Float%20%28single-precision%29))
  (Variables|Default|SetMaxNumSections (Math|Float|Truncate (/ Length (Variables|Default|GetSectionLength)))))