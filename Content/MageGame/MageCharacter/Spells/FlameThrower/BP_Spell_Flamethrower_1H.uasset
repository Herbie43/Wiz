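; One-handed flamethrower spell for the mage, streaming flame from a supplied spawn point while firing.
; Fire stores that component and opens a Tick gate, which attaches the flame particle through a DoOnce and uses a Delay to throttle spawning of flame projectiles.
; StopFire calls Release, deactivates the particle and closes the gate.
; Each gated tick also line traces from the owner's first-person camera, but the result is unused.
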(event Custom|Fire
  (params (SpawnPoint :type Scene%20Component%20Object%20Reference) (NewParam :type Boolean))
  (bind _spellowner (Variables|Default|GetSpellOwner))
  (bind _asbp_mage_base (Utilities|Casting|CastToBP_MageBase _spellowner))
  (bind _fp_camera (Variables|/Game/MageGame/MageCharacter/BP_MageBase.BP_MageBase_C|GetFP_Camera _asbp_mage_base))
  (bind _returnvalue (Math|Vector|GetForwardVector _fp_camera))
  (Variables|Default|SetAttachedComponent SpawnPoint)
  (Utilities|FlowControl|Gate true) ; enters at Open
)

(event Custom|Release
  (Utilities|FlowControl|DoOnce false
    (:Completed
      (bind _returnvalue (Effects|SpawnEmitterAttached "/Game/Effects/Flamethrower/P_Flamethrower_1H.P_Flamethrower_1H" (Variables|Default|GetAttachedComponent) "None"))
      (Variables|Default|SetParticleSystem _returnvalue))))

(event Custom|StopFire
  (bind _attachedcomponent (Variables|Default|GetAttachedComponent))
  (bind _spellowner (Variables|Default|GetSpellOwner))
  (bind _asbp_mage_base (Utilities|Casting|CastToBP_MageBase _spellowner))
  (bind _fp_camera (Variables|/Game/MageGame/MageCharacter/BP_MageBase.BP_MageBase_C|GetFP_Camera _asbp_mage_base))
  (bind _returnvalue (Math|Vector|GetForwardVector _fp_camera))
  (CallFunction|Release)
  (Components|Activation|Deactivate (Variables|Default|GetParticleSystem))
  (Utilities|FlowControl|Gate true) ; enters at Close
)

(event EventBeginPlay
  (|CallParentFunction) ; This node is disabled and will not be called.\nDrag off pins to build functionality.
)

(event Collision|EventActorBeginOverlap
  (params (OtherActor :type Actor%20Object%20Reference))
  (|CallParentFunction OtherActor) ; This node is disabled and will not be called.\nDrag off pins to build functionality.
)

(event EventTick
  (params (DeltaSeconds :type Float%20%28single-precision%29))
  (bind _attachedcomponent (Variables|Default|GetAttachedComponent))
  (bind _spellowner (Variables|Default|GetSpellOwner))
  (bind _asbp_mage_base (Utilities|Casting|CastToBP_MageBase _spellowner))
  (bind _fp_camera (Variables|/Game/MageGame/MageCharacter/BP_MageBase.BP_MageBase_C|GetFP_Camera _asbp_mage_base))
  (bind _returnvalue (Math|Vector|GetForwardVector _fp_camera))
  (|CallParentFunction DeltaSeconds)
  (Utilities|FlowControl|Sequence
    (:then_1
      (Utilities|FlowControl|Gate true
        (:Exit
          (Collision|LineTraceByChannel (+ (Transformation|GetWorldLocation _fp_camera) _returnvalue) (* _returnvalue 1e+03) "TraceTypeQuery1" false (Utilities|Array|MakeArray _spellowner) "None")
          (Utilities|FlowControl|Sequence
            (:then_0
              (Utilities|FlowControl|DoOnce false
                (:Completed
                  (bind _returnvalue_2 (Effects|SpawnEmitterAttached "/Game/Effects/Flamethrower/P_Flamethrower_1H.P_Flamethrower_1H" (Variables|Default|GetAttachedComponent) "None"))
                  (Variables|Default|SetParticleSystem _returnvalue_2))))
            (:then_1
              (Utilities|FlowControl|Delay 0.1)
              (bind _returnvalue_3 (Game|SpawnActorfromClass "/Game/MageGame/MageCharacter/Spells/FlameThrower/BP_Flame_Projectile.BP_Flame_Projectile_C" (Math|Transform|MakeTransform (Transformation|GetWorldLocation _attachedcomponent) (Transformation|GetWorldRotation _attachedcomponent)) "Undefined" 0 (Variables|Default|GetSpellOwner) 0))
              (Variables|Default|SetProjectileRef _returnvalue_3))))))))

(fn ConstructionScript
  (|CallParentFunction))