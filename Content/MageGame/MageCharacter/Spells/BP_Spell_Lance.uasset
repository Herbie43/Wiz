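; BP_Spell_Lance is a mage spell Blueprint for a fast Lance with an ice explosion effect and no morphs.
; It is a data-only style child: its construction script runs the parent's, then overrides range and speed, clears the morph list and sets the explosion particle.
; The event graph holds only disabled default events, so any runtime behavior comes from the parent class.
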(event EventBeginPlay
  (|CallParentFunction) ; This node is disabled and will not be called.\nDrag off pins to build functionality.
)

(event Collision|EventActorBeginOverlap
  (params (OtherActor :type Actor%20Object%20Reference))
  (|CallParentFunction OtherActor) ; This node is disabled and will not be called.\nDrag off pins to build functionality.
)

(event EventTick
  (params (DeltaSeconds :type Float%20%28single-precision%29))
  (|CallParentFunction DeltaSeconds) ; This node is disabled and will not be called.\nDrag off pins to build functionality.
)

(fn ConstructionScript
  (|CallParentFunction)
  (Variables|Default|SetSpellRange 4e+03)
  (Variables|Default|SetSpeed 4e+03)
  (Utilities|Array|Clear (Variables|Default|GetMorphs))
  (Variables|Default|SetHasMorphs false)
  (Variables|Default|SetExplosionEffect "/Game/MageGame/MageCharacter/Spells/Explosions/P_Explosion_Ice.P_Explosion_Ice"))