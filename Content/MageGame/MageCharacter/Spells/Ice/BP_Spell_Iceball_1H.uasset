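; BP_Spell_Iceball_1H is the one-handed iceball spell, a data-only style child of a parent spell Blueprint.
; Its construction script sets the magic and spell type enums, ice explosion effect, impact sound and half-size maximum scale, then calls the parent construction script.
; It adds no runtime logic of its own, as its event graph holds only disabled placeholder events.
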(event EventBeginPlay
  (|CallParentFunction) ; This node is disabled and will not be called.\nDrag off pins to build functionality.
)

(event Collision|EventActorBeginOverlap
  (params (OtherActor :type Actor%20Object%20Reference))
  (|CallParentFunction OtherActor) ; This node is disabled and will not be called.\nDrag off pins to build functionality.
)

(event EventTick
  (params (DeltaSeconds :type Float%20%28single-precision%29))
  (|CallParentFunction DeltaSeconds) ; This node is disabled and will not be called.\nDrag off pins to build functionality.
)

(fn ConstructionScript
  (Variables|Default|SetMagicType "NewEnumerator1")
  (Variables|Default|SetSpellType "NewEnumerator5")
  (Variables|Default|SetExplosionEffect "/Game/MageGame/MageCharacter/Spells/Explosions/P_Explosion_Ice.P_Explosion_Ice")
  (Variables|Default|SetDestroyedSound "/Game/IceFrostMagic1_SoundFXPack/wavs/Spells/Impact/Ice/Magic_Spells_Impact_Ice06.Magic_Spells_Impact_Ice06")
  (Variables|Default|SetMaxScale "0.500000,0.500000,0.500000")
  (|CallParentFunction))