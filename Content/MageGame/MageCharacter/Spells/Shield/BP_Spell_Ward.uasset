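; BP_Spell_Ward is a shield spell for mages that intercepts other spells with a capsule collider.
; On capsule overlap with a BP_SpellBase actor, it destroys that spell and itself, printing both names.
; On a capsule hit by a valid spell, it passes a value derived from that spell's current damage to ChangeMana on the owning BP_MageBase.
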(event OnComponentHit(Capsule)
  (params (HitComponent :type Primitive%20Component%20Object%20Reference) (OtherActor :type Actor%20Object%20Reference) (OtherComp :type Primitive%20Component%20Object%20Reference) (NormalImpulse :type Vector :default "0, 0, 0") (Hit :type Hit%20Result%20Structure%20%28by%20ref%29))
  (bind _asbp_spell_base (Utilities|Casting|CastToBP_SpellBase OtherActor))
  (Utilities|IsValid _asbp_spell_base
    (:Is%20Valid
      (bind _asbp_mage_base (Utilities|Casting|CastToBP_MageBase (Components|GetOwner)))
      (bind _result (Math|Float|NegateFloat (Variables|/Game/MageGame/MageCharacter/Spells/BP_SpellBase.BP_SpellBase_C|GetDamage_Current _asbp_spell_base))
        (:%20%20
          (Default|ChangeMana _asbp_mage_base _result))))))

(event OnComponentBeginOverlap(Capsule)
  (params (OverlappedComponent :type Primitive%20Component%20Object%20Reference) (OtherActor :type Actor%20Object%20Reference) (OtherComp :type Primitive%20Component%20Object%20Reference) (OtherBodyIndex :type Integer) (bFromSweep :type Boolean) (SweepResult :type Hit%20Result%20Structure%20%28by%20ref%29))
  (bind _self self)
  (bind _asbp_spell_base (Utilities|Casting|CastToBP_SpellBase OtherActor))
  (Actor|DestroyActor _asbp_spell_base)
  (Development|PrintString (Utilities|GetDisplayName _asbp_spell_base))
  (Actor|DestroyActor _self)
  (Development|PrintString (Utilities|GetDisplayName _self)))

(event EventBeginPlay
  (|CallParentFunction) ; This node is disabled and will not be called.\nDrag off pins to build functionality.
)

(event Collision|EventActorBeginOverlap
  (params (OtherActor :type Actor%20Object%20Reference))
  (|CallParentFunction OtherActor) ; This node is disabled and will not be called.\nDrag off pins to build functionality.
)

(event EventTick
  (params (DeltaSeconds :type Float%20%28single-precision%29))
  (|CallParentFunction DeltaSeconds) ; This node is disabled and will not be called.\nDrag off pins to build functionality.
)

(fn ConstructionScript
  (|CallParentFunction))