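; BP_SpellShield is a mage's shield spell that intercepts other spells.
; Capsule overlap with a spell destroys both, while a blocking hit or TakeHit converts damage into a mana change on the owning mage.
; Fire stores the spawn point and opens a gate for a per-tick camera line trace, whose result is unused and whose end point omits the camera location.
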(event OnComponentHit(Capsule)
  (params (HitComponent :type Primitive%20Component%20Object%20Reference) (OtherActor :type Actor%20Object%20Reference) (OtherComp :type Primitive%20Component%20Object%20Reference) (NormalImpulse :type Vector :default "0, 0, 0") (Hit :type Hit%20Result%20Structure%20%28by%20ref%29))
  (bind _asbp_spell_base (Utilities|Casting|CastToBP_SpellBase OtherActor))
  (Utilities|IsValid _asbp_spell_base
    (:Is%20Valid
      (bind _asbp_mage_base (Utilities|Casting|CastToBP_MageBase (Components|GetOwner)))
      (bind _result (Math|Float|NegateFloat (Variables|/Game/MageGame/MageCharacter/Spells/BP_SpellBase.BP_SpellBase_C|GetDamage_Current _asbp_spell_base))
        (:%20%20
          (Default|ChangeMana _asbp_mage_base _result))))))

(event OnComponentBeginOverlap(Capsule)
  (params (OverlappedComponent :type Primitive%20Component%20Object%20Reference) (OtherActor :type Actor%20Object%20Reference) (OtherComp :type Primitive%20Component%20Object%20Reference) (OtherBodyIndex :type Integer) (bFromSweep :type Boolean) (SweepResult :type Hit%20Result%20Structure%20%28by%20ref%29))
  (bind _self self)
  (bind _asbp_spell_base (Utilities|Casting|CastToBP_SpellBase OtherActor))
  (Actor|DestroyActor _asbp_spell_base)
  (Development|PrintString (Utilities|GetDisplayName _asbp_spell_base))
  (Actor|DestroyActor _self)
  (Development|PrintString (Utilities|GetDisplayName _self)))

(event Custom|Fire
  (params (SpawnPoint :type Scene%20Component%20Object%20Reference))
  (bind _spellowner (Variables|Default|GetSpellOwner))
  (bind _asbp_mage_base (Utilities|Casting|CastToBP_MageBase _spellowner))
  (bind _fp_camera (Variables|/Game/MageGame/MageCharacter/BP_MageBase.BP_MageBase_C|GetFP_Camera _asbp_mage_base))
  (bind _returnvalue (Math|Vector|GetForwardVector _fp_camera))
  (Variables|Default|SetAttachedComponent SpawnPoint)
  (Utilities|FlowControl|Gate true) ; enters at Open
)

(event EventBeginPlay)

(event Collision|EventActorBeginOverlap
  (params (OtherActor :type Actor%20Object%20Reference)))

(event EventTick
  (params (DeltaSeconds :type Float%20%28single-precision%29))
  (bind _spellowner (Variables|Default|GetSpellOwner))
  (bind _asbp_mage_base (Utilities|Casting|CastToBP_MageBase _spellowner))
  (bind _fp_camera (Variables|/Game/MageGame/MageCharacter/BP_MageBase.BP_MageBase_C|GetFP_Camera _asbp_mage_base))
  (bind _returnvalue (Math|Vector|GetForwardVector _fp_camera))
  (Utilities|FlowControl|Sequence
    (:then_1
      (Utilities|FlowControl|Gate true
        (:Exit
          (Collision|LineTraceByChannel (+ (Transformation|GetWorldLocation _fp_camera) _returnvalue) (* _returnvalue 1e+02) "TraceTypeQuery1" false (Utilities|Array|MakeArray _spellowner) "None"))))))

(fn ConstructionScript)

(fn TakeHit
  (params (Amount :type Float%20%28single-precision%29))
  (Development|PrintString (Utilities|String|Append "Shield hit for " (Utilities|String|ToString(Float) Amount) " damage"))
  (bind _asbp_mage_base (Utilities|Casting|CastToBP_MageBase (Components|GetOwner)))
  (bind _result (Math|Float|NegateFloat Amount)
    (:%20%20
      (Default|ChangeMana _asbp_mage_base _result))))

(fn DestroySelf
  (Actor|DestroyActor))