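; Two-handed lightning bolt spell that fires an arc from the mage and applies a Conduit debuff to a struck mage.
; On release it line-traces along first-person camera forward, stores the hit and resets charge state.
; Arcing spawns a BP_SpawnedArc fed by an arc struct, with branching driven by the target's existing Conduit debuff.
; Location Logic selects endpoints from vectors, objects or random mesh vertices; SetSpellTarget also triggers arcing.
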(event Custom|SetSpellTarget
  (params (NewParam :type Vector))
  (Variables|Arc|SetDestination NewParam)
  (CallFunction|Arcing))

(event Custom|Arcing
  (bind _returnvalue (Transformation|GetActorLocation))
  (bind _arcstruct (Variables|Arc|GetArcStruct))
  (bind (_distance _boltcolor _isbranch _allowbranches _branchlimit _priorhitloc _priorhitnormal _playrate _customvectors _origin _dest _noisescale _noisespeed _hitplayer) (Utilities|Struct|BreakArcValues _arcstruct))
  (bind _returnvalue_2 (Game|SpawnActorfromClass "/Game/ThirdPersonBP/Lightning/BP_SpawnedArc.BP_SpawnedArc_C" (Math|Transform|MakeTransform (Math|Vector|MakeVector (.x _returnvalue) (.y _returnvalue) (- (.z _returnvalue) 1e+01)) (Transformation|GetActorRotation) "1,1,1") "Undefined" self (Variables|Arc|GetMoveable?) 0))
  (|SetupArcStruct)
  (switch Utilities|FlowControl|Switch|SwitchonArcStyle (Variables|Arc|GetStyleSelector)
    (:NewEnumerator1
      (|LocationLogic)
      (Default|Spawn _returnvalue_2 (Utilities|Struct|MakeArcValues _distance _boltcolor _isbranch _allowbranches _branchlimit _priorhitloc _priorhitnormal _playrate true _origin _dest _noisescale _noisespeed _hitplayer))
      (bind _asbp_mage_base (Utilities|Casting|CastToBP_MageBase (Variables|Default|GetHitActor)))
      (Utilities|Array|AddUnique (Variables|/Game/MageGame/MageCharacter/BP_MageBase.BP_MageBase_C|GetDebuffs _asbp_mage_base) "(TagName=\"Conduit\")"))))

(event Custom|spell%20multi%20stop
  (params (NewParam :type Particle%20System%20Component%20Object%20Reference))
  (Components|Activation|Deactivate (Variables|Default|GetSpellEffect)))

(event EventBeginPlay
  (|CallParentFunction))

(event Collision|EventActorBeginOverlap
  (params (OtherActor :type Actor%20Object%20Reference))
  (|CallParentFunction OtherActor) ; This node is disabled and will not be called.\nDrag off pins to build functionality.
)

(event EventTick
  (params (DeltaSeconds :type Float%20%28single-precision%29))
  (|CallParentFunction DeltaSeconds) ; This node is disabled and will not be called.\nDrag off pins to build functionality.
)

(event EventSpellReleased
  (bind _spellowner (Variables|Default|GetSpellOwner))
  (bind _asbp_mage_base (Utilities|Casting|CastToBP_MageBase _spellowner))
  (bind _projectilespawnlocation (Variables|/Game/MageGame/MageCharacter/BP_MageBase.BP_MageBase_C|GetProjectileSpawnLocation _asbp_mage_base))
  (bind _returnvalue (Transformation|GetWorldLocation _projectilespawnlocation))
  (CallFunction|SpellMultiStop (Variables|Default|GetSpellEffect))
  (Variables|Arc|SetOrigin _returnvalue)
  (bind (_outhit _returnvalue_2) (Collision|LineTraceByChannel _returnvalue (+ _returnvalue (* (Variables|/Game/MageGame/MageCharacter/BP_MageBase.BP_MageBase_C|GetFPCamForward _asbp_mage_base) (Variables|Default|GetSpellRange))) "TraceTypeQuery1" false (Utilities|Array|MakeArray (Variables|Default|GetSpellOwner)) "None"))
  (if _returnvalue_2
    (Utilities|Casting|CastToBP_MageBase (.HitActor (Collision|BreakHitResult _outhit))
      (:then
        (Variables|Default|SetHitActor (.HitActor (Collision|BreakHitResult _outhit)))
        (Variables|Arc|SetHitLocation (.Location (Collision|BreakHitResult _outhit)))
        (Variables|Arc|SetHitNormal (.ImpactNormal (Collision|BreakHitResult _outhit)))
        (CallFunction|Arcing))
      (:CastFailed
        (Variables|Arc|SetHitLocation (.Location (Collision|BreakHitResult _outhit)))
        (Variables|Arc|SetHitNormal (.ImpactNormal (Collision|BreakHitResult _outhit)))
        (CallFunction|Arcing)))
    (else
      (CallFunction|Arcing)))
  (CallFunction|StopOverload)
  (CallFunction|StopMaxCharge)
  (CallFunction|StopCharging)
  (CallFunction|ResetCastVariables))

(fn ConstructionScript
  (|CallParentFunction)
  (Rendering|Components|Light|SetLightColor (Variables|Default|GetPointLight) (Variables|Arc|GetArcColor) true))