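; Flame projectile for the mage's fire spells that damages what it hits and expires after a set Length.
; Each tick, a very short sphere trace on the Visibility channel at the collision sphere finds blocking hits.
; A hit applies point damage credited to the owning mage's controller, then destroys the projectile; elemental damage is still a TODO.
; The sphere's own hit event only prints the other actor's name, and its overlap event does nothing.
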(event OnComponentActivated(ProjectileMovement)
  (params (Component :type Actor%20Component%20Object%20Reference) (bReset :type Boolean))
  (Utilities|FlowControl|Delay (Variables|Default|GetLength))
  (Actor|DestroyActor))

(event OnComponentHit(Sphere)
  (params (HitComponent :type Primitive%20Component%20Object%20Reference) (OtherActor :type Actor%20Object%20Reference) (OtherComp :type Primitive%20Component%20Object%20Reference) (NormalImpulse :type Vector :default "0, 0, 0") (Hit :type Hit%20Result%20Structure%20%28by%20ref%29))
  (Development|PrintString (Utilities|GetDisplayName OtherActor)))

(event OnComponentBeginOverlap(Sphere)
  (params (OverlappedComponent :type Primitive%20Component%20Object%20Reference) (OtherActor :type Actor%20Object%20Reference) (OtherComp :type Primitive%20Component%20Object%20Reference) (OtherBodyIndex :type Integer) (bFromSweep :type Boolean) (SweepResult :type Hit%20Result%20Structure%20%28by%20ref%29))
  (if (== OtherActor (Variables|Default|GetSpellOwner))
    _))

(event EventBeginPlay)

(event Collision|EventActorBeginOverlap
  (params (OtherActor :type Actor%20Object%20Reference)))

(event EventTick
  (params (DeltaSeconds :type Float%20%28single-precision%29))
  (CallFunction|TraceforDamage))

(event EventDestroyed)

(fn ConstructionScript)

(fn TraceforDamage
  (bind _sphere (Variables|Default|GetSphere))
  (bind _returnvalue (Transformation|GetWorldLocation _sphere))
  (bind _outhit (Collision|SphereTraceByChannel _returnvalue (+ _returnvalue "1.000000,1.000000,1.000000") 0.0 "TraceTypeQuery1" false 0 "None"))
  (if (.bBlockingHit (Collision|BreakHitResult _outhit))
    ;[1 1 1] TODO: Elemental Damage here
    (Utilities|FlowControl|Sequence
      (:then_0
        (Game|Damage|ApplyPointDamage (.HitActor (Collision|BreakHitResult _outhit)) (Variables|Default|GetBaseDamage) (.ImpactPoint (Collision|BreakHitResult _outhit)) _outhit (Pawn|GetController (.AsBP%20Mage%20Base (Utilities|Casting|CastToBP_MageBase (Variables|Default|GetSpellOwner)))) self)
        (Actor|DestroyActor)))))