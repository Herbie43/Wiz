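; Two-handed fire spell for the mage that channels a stream of flames after charging.
; Cast time is linearly scaled into a release duration on the server.
; Once released, Tick fires flame projectiles, throttled by a short delay, toward a point ahead of the first-person camera while the flame effect follows its attach component.
; When the countdown expires, it deactivates the effect, resets casting and ends the mage's channel.
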(event Custom|Fire
  (bind _spellowner (Variables|Default|GetSpellOwner))
  (bind _startlocation (Variables|Default|GetStartLocation))
  (bind _asbp_mage_base (Utilities|Casting|CastToBP_MageBase _spellowner))
  (bind _fpcamlocation (Variables|/Game/MageGame/MageCharacter/BP_MageBase.BP_MageBase_C|GetFPCamLocation _asbp_mage_base))
  (bind _fpcamforward (Variables|/Game/MageGame/MageCharacter/BP_MageBase.BP_MageBase_C|GetFPCamForward _asbp_mage_base))
  (bind _returnvalue (* _fpcamforward 1e+03))
  (bind _returnvalue_2 (+ _fpcamlocation _returnvalue))
  (bind _returnvalue_3 (Math|Rotator|FindLookatRotation _startlocation _returnvalue_2))
  (Utilities|FlowControl|Sequence
    (:then_0
      (bind (_outhit _returnvalue_4) (Collision|LineTraceByChannel _fpcamlocation _returnvalue_2 "TraceTypeQuery1" false (Utilities|Array|MakeArray self _spellowner) "None"))
      (CallFunction|UpdateSpawnLocation)
      (Utilities|FlowControl|Sequence
        (:then_0
          (CallFunction|ReleaseMulti (Variables|Default|GetSpellEffect) (Transformation|GetActorTransform)))
        (:then_1
          (Utilities|FlowControl|Delay 0.1)
          (if _returnvalue_4
            (Variables|Default|SetShootTo (Math|Transform|MakeTransform _startlocation _returnvalue_3))
            (else
              (Variables|Default|SetShootTo (Math|Transform|MakeTransform _startlocation _returnvalue_3))))
          (bind _returnvalue_5 (Game|SpawnActorfromClass "/Game/MageGame/MageCharacter/Spells/Fire/Flames/BP_Flame_Projectile.BP_Flame_Projectile_C" (Variables|Default|GetShootTo) "Undefined" 0 (Variables|Default|GetSpellOwner) 0.4 1e+01 0))
          (Variables|Default|SetProjectileRef _returnvalue_5)
          (CallFunction|UpdateFlames (Transformation|GetWorldTransform (Variables|Default|GetAttachedComponent)) (Variables|Default|GetSpellEffect))
          (for _array_element (Variables|Default|GetIgnoredComponents)
            (Collision|IgnoreActorwhenMoving _array_element _returnvalue_5 true))
          (bind _output_get (Variables|Default|SetReleaseTime (- (Variables|Default|GetReleaseTime) (stale EventTick DeltaSeconds))))
          (Development|PrintString (Utilities|String|ToString(Float) _output_get) true true "(R=0.359550,G=1.000000,B=0.000000,A=1.000000)" 1e+03)
          (if (<= _output_get 0.0)
            (CallFunction|StopFire)))))
    (:then_1
      (Utilities|FlowControl|Gate true))))

(event Custom|StopFire
  (bind _spelleffect (Variables|Default|GetSpellEffect))
  (Utilities|IsValid _spelleffect
    (:Is%20Valid
      (Components|Activation|Deactivate _spelleffect)
      (CallFunction|PlayAudio (Variables|Default|GetCastAudio))
      (CallFunction|StopOverload)
      (CallFunction|StopMaxCharge)
      (CallFunction|StopCharging)
      (CallFunction|ResetCastVariables)
      (bind _asbp_mage_base (Utilities|Casting|CastToBP_MageBase (Variables|Default|GetSpellOwner)))
      (Default|StopChannelingSpell _asbp_mage_base))))

(event Custom|UpdateFlames
  (params (NewParam :type Transform) (Target :type Scene%20Component%20Object%20Reference))
  (Transformation|SetWorldTransform Target NewParam false false))

(event Custom|StartRelease
  (params (Spawn%20Point :type Scene%20Component%20Object%20Reference))
  (Variables|Default|SetAttachedComponent Spawn%20Point)
  (Variables|Default|SetIsReleased? true)
  (Variables|Default|SetIsCharging? false)
  (Utilities|FlowControl|Gate true) ; enters at Open
)

(event Custom|Release_Multi
  (params (Target :type Actor%20Component%20Object%20Reference) (NewTransform :type Transform%20%28by%20ref%29))
  (Utilities|FlowControl|DoOnce false
    (:Completed
      (Components|Activation|Activate Target false)
      (bind _asscene_component (Utilities|Casting|CastToSceneComponent Target))
      (Transformation|SetWorldTransform _asscene_component NewTransform false false))))

(event EventBeginPlay
  (|CallParentFunction) ; This node is disabled and will not be called.\nDrag off pins to build functionality.
)

(event Collision|EventActorBeginOverlap
  (params (OtherActor :type Actor%20Object%20Reference))
  (|CallParentFunction OtherActor) ; This node is disabled and will not be called.\nDrag off pins to build functionality.
)

(event EventTick
  (params (DeltaSeconds :type Float%20%28single-precision%29))
  (|CallParentFunction DeltaSeconds)
  (if (Variables|Default|GetIsReleased?)
    (CallFunction|Fire)))

(event EventHandleReleaseTimeonServer
  (bind _result (CallFunction|ScaleLinearRange (Variables|Default|GetCurrentCastTime) (Variables|Default|GetMinimumCastTime) (Variables|Default|GetCastTime) (Variables|Default|GetReleaseTimeMin) (Variables|Default|GetReleaseTimeMax)))
  (bind _output_get (Variables|Default|SetReleaseTime (* _result (Variables|Default|GetReleaseTimeScalar))))
  (Development|PrintString (Utilities|String|ToString(Float) _output_get) true true "(R=0.000000,G=0.660000,B=1.000000,A=1.000000)" 1e+03))

(event EventChargeSpell
  (if (Variables|Default|GetIsActivated?)
    (if (Variables|Default|GetIsCharging?)
      (CallFunction|EnterChargeGate))
    (else
      (CallFunction|ActivateSpell))))

(fn ConstructionScript
  (|CallParentFunction))

(fn UpdateSpawnLocation
  (Variables|Default|SetStartLocation (Variables|/Game/MageGame/MageCharacter/BP_MageBase.BP_MageBase_C|Get2HSpawnLocation (.AsBP%20Mage%20Base (Utilities|Casting|CastToBP_MageBase (Variables|Default|GetSpellOwner))))))