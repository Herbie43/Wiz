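; Two-handed Fireball spell projectile for mages that explodes in radial damage and supports overload charging.
; Overlaps skip the instigator and dead mages, deal fixed-radius damage and add damage-over-time to mages.
; Blocking hits spawn an explosion and debug sphere, using a damage radius of sphere size plus overload charge.
; Overloading stops the caster's charging and detonates maximum damage at their projectile spawn point, destroying the spell.
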(event OnComponentBeginOverlap(Sphere)
  (params (OverlappedComponent :type Primitive%20Component%20Object%20Reference) (OtherActor :type Actor%20Object%20Reference) (OtherComp :type Primitive%20Component%20Object%20Reference) (OtherBodyIndex :type Integer) (bFromSweep :type Boolean) (SweepResult :type Hit%20Result%20Structure%20%28by%20ref%29))
  (bind (_bblockinghit _binitialoverlap _time _distance _location _impactpoint _normal _impactnormal _physmat _hitactor) (Collision|BreakHitResult SweepResult))
  (bind _self self)
  (bind _sphere (Variables|Default|GetSphere))
  (bind _damage_current (Variables|Default|GetDamage_Current))
  (bind _spellowner (Variables|Default|GetSpellOwner))
  (bind _returnvalue (Components|Sphere|GetScaledSphereRadius _sphere))
  (bind _instigator (Variables|/Script/Engine.Actor|GetInstigator _spellowner))
  (bind _returnvalue_2 (Pawn|GetController _instigator))
  (if (not (== OtherActor (Game|GetInstigator)))
    (bind _asbp_mage_base (Utilities|Casting|CastToBP_MageBase OtherActor)
      (:then
        (if (not (Variables|/Game/MageGame/MageCharacter/BP_MageBase.BP_MageBase_C|GetIsDead? _asbp_mage_base))
          (Development|PrintString (Utilities|GetDisplayName OtherActor) :!label _label)
          (if (> (Variables|Default|GetOverloadCharge) 0.0)
            (Variables|Default|SetExplosionRadius (+ (Variables|Default|GetOverloadCharge) _returnvalue))
            (else
              (Variables|Default|SetExplosionRadius _returnvalue)))
          (bind _asbp_mage_base_2 (Utilities|Casting|CastToBP_MageBase _hitactor)
            (:then
              (Game|Damage|ApplyRadialDamage _damage_current _impactpoint 2e+02 0 0 _self _returnvalue_2 false "ECC_Visibility")
              (Default|ApplyDoTonServer _asbp_mage_base_2 1e+01 5.0 (.AsPlayer%20Controller (Utilities|Casting|CastToPlayerController _returnvalue_2)) self))
            (:CastFailed
              (Game|Damage|ApplyRadialDamage _damage_current _impactpoint 2e+02 0 0 _self 0 false "ECC_Visibility")))
          (Development|PrintString (Utilities|String|Append (Utilities|String|ToString(Float) (Components|Sphere|GetScaledSphereRadius (Variables|Default|GetSphere))) "explosion radius") true true "(R=0.000000,G=0.660000,B=1.000000,A=1.000000)" 2e+01)
          (Actor|DestroyActor)))
      (:CastFailed
        (goto _label)))))

(event OnComponentHit(Sphere)
  (params (HitComponent :type Primitive%20Component%20Object%20Reference) (OtherActor :type Actor%20Object%20Reference) (OtherComp :type Primitive%20Component%20Object%20Reference) (NormalImpulse :type Vector :default "0, 0, 0") (Hit :type Hit%20Result%20Structure%20%28by%20ref%29))
  (bind _returnvalue (Components|GetOwner))
  (bind (_bblockinghit _binitialoverlap _time _distance _location _impactpoint _normal _impactnormal _physmat _hitactor) (Collision|BreakHitResult Hit))
  (bind _self self)
  (bind _sphere (Variables|Default|GetSphere))
  (bind _damage_current (Variables|Default|GetDamage_Current))
  (bind _returnvalue_2 (Components|Sphere|GetScaledSphereRadius _sphere))
  (if (not (== _hitactor _returnvalue))
    (Game|SpawnActorfromClass "/Game/StarterContent/Blueprints/Blueprint_Effect_Explosion.Blueprint_Effect_Explosion_C" (Math|Transform|MakeTransform _impactpoint (.rotation (Transformation|GetActorTransform _hitactor)) "1,1,1") "Undefined" _returnvalue 0)
    (if (> (Variables|Default|GetOverloadCharge) 0.0)
      (Variables|Default|SetExplosionRadius (+ (Variables|Default|GetOverloadCharge) _returnvalue_2))
      (else
        (Variables|Default|SetExplosionRadius _returnvalue_2)))
    (bind _asbp_mage_base (Utilities|Casting|CastToBP_MageBase _returnvalue)
      (:then
        (Game|Damage|ApplyRadialDamage _damage_current _impactpoint (Variables|Default|GetExplosionRadius) 0 0 _self (Pawn|GetController _asbp_mage_base) false "ECC_Visibility"))
      (:CastFailed
        (Game|Damage|ApplyRadialDamage _damage_current _impactpoint (Variables|Default|GetExplosionRadius) 0 0 _self 0 false "ECC_Visibility")))
    (Game|SpawnActorfromClass "/Game/MageGame/DebugObjects/DebugSphere.DebugSphere_C" (Math|Transform|MakeTransform _impactpoint "0, 0, 0" "1,1,1") "Undefined" 0 (Variables|Default|GetExplosionRadius) 0)
    (Actor|DestroyActor)))

(event EventBeginPlay
  (|CallParentFunction) ; This node is disabled and will not be called.\nDrag off pins to build functionality.
)

(event Collision|EventActorBeginOverlap
  (params (OtherActor :type Actor%20Object%20Reference))
  (|CallParentFunction OtherActor) ; This node is disabled and will not be called.\nDrag off pins to build functionality.
)

(event EventTick
  (params (DeltaSeconds :type Float%20%28single-precision%29))
  (|CallParentFunction DeltaSeconds))

(event EventApplyOverloadChange
  (bind _output_get (Variables|Default|SetExplosionRadius (+ (Variables|Default|GetExplosionRadius) (Variables|Default|GetOverloadChargeRate))))
  (Development|PrintString (Utilities|String|Append (Utilities|String|ToString(Float) _output_get) "explosion raidus!!!!!")))

(event EventSpellOverloaded
  (bind _asbp_mage_base (Utilities|Casting|CastToBP_MageBase (Variables|Default|GetSpellOwner)))
  (Default|StopCharging _asbp_mage_base)
  (Game|Damage|ApplyRadialDamage (Variables|Default|GetDamage_Max) (Transformation|GetWorldLocation (Variables|/Game/MageGame/MageCharacter/BP_MageBase.BP_MageBase_C|GetProjectileSpawnLocation _asbp_mage_base)) 2e+02 0 0 self (Pawn|GetController (.AsBP%20Mage%20Base (Utilities|Casting|CastToBP_MageBase (Variables|Default|GetSpellOwner)))) false "ECC_Visibility")
  (CallFunction|StopOverloadEffect)
  (CallFunction|SpellOverloadedEffect)
  (Actor|DestroyActor))

(fn ConstructionScript
  (|CallParentFunction)
  (Variables|Default|SetDestroyedSound "/Game/StarterContent/Audio/Explosion01.Explosion01")
  (Variables|Default|SetExplosionEffect "/Game/StarterContent/Particles/P_Explosion.P_Explosion"))