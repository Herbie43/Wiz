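; Two-handed flamethrower spell for the mage: emits an attached flame effect and fires a stream of projectiles while active.
; Fire and StopFire open and close a Tick gate, with a short Delay throttling BP_Flame_Projectile spawns from the mage's two-hand spawn location.
; Projectiles and particles aim at a point ahead of the first-person camera; both line-trace branches use this point, ignoring the impact.
; Listed components ignore each new projectile when moving.
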(event Custom|Fire
  (params (SpawnPoint :type Scene%20Component%20Object%20Reference))
  (bind _spellowner (Variables|Default|GetSpellOwner))
  (bind _startlocation (Variables|Default|GetStartLocation))
  (bind _asbp_mage_base (Utilities|Casting|CastToBP_MageBase _spellowner))
  (bind _fpcamlocation (Variables|/Game/MageGame/MageCharacter/BP_MageBase.BP_MageBase_C|GetFPCamLocation _asbp_mage_base))
  (bind _fpcamforward (Variables|/Game/MageGame/MageCharacter/BP_MageBase.BP_MageBase_C|GetFPCamForward _asbp_mage_base))
  (bind _returnvalue (* _fpcamforward 1e+03))
  (bind _returnvalue_2 (+ _fpcamlocation _returnvalue))
  (bind _returnvalue_3 (Math|Rotator|FindLookatRotation _startlocation _returnvalue_2))
  (Variables|Default|SetAttachedComponent SpawnPoint)
  (Utilities|FlowControl|Gate true) ; enters at Open
)

(event Custom|Release
  (Utilities|FlowControl|DoOnce false
    (:Completed
      (bind _returnvalue (Effects|SpawnEmitterAttached "/Game/Effects/Flamethrower/P_Flamethrower_2H.P_Flamethrower_2H" (Variables|Default|GetAttachedComponent) "None"))
      (Variables|Default|SetParticleSystem _returnvalue))))

(event Custom|StopFire
  (bind _spellowner (Variables|Default|GetSpellOwner))
  (bind _startlocation (Variables|Default|GetStartLocation))
  (bind _particlesystem (Variables|Default|GetParticleSystem))
  (bind _asbp_mage_base (Utilities|Casting|CastToBP_MageBase _spellowner))
  (bind _fpcamlocation (Variables|/Game/MageGame/MageCharacter/BP_MageBase.BP_MageBase_C|GetFPCamLocation _asbp_mage_base))
  (bind _fpcamforward (Variables|/Game/MageGame/MageCharacter/BP_MageBase.BP_MageBase_C|GetFPCamForward _asbp_mage_base))
  (bind _returnvalue (* _fpcamforward 1e+03))
  (bind _returnvalue_2 (+ _fpcamlocation _returnvalue))
  (bind _returnvalue_3 (Math|Rotator|FindLookatRotation _startlocation _returnvalue_2))
  (CallFunction|Release)
  (Utilities|IsValid _particlesystem
    (:Is%20Valid
      (Components|Activation|Deactivate _particlesystem)
      (Utilities|FlowControl|Gate true) ; enters at Close
    )))

(event Custom|UpdateFlames
  (params (NewParam :type Transform))
  (Transformation|SetWorldTransform (Variables|Default|GetParticleSystem) NewParam false false))

(event EventBeginPlay
  (|CallParentFunction) ; This node is disabled and will not be called.\nDrag off pins to build functionality.
)

(event Collision|EventActorBeginOverlap
  (params (OtherActor :type Actor%20Object%20Reference))
  (|CallParentFunction OtherActor) ; This node is disabled and will not be called.\nDrag off pins to build functionality.
)

(event EventTick
  (params (DeltaSeconds :type Float%20%28single-precision%29))
  (bind _spellowner (Variables|Default|GetSpellOwner))
  (bind _startlocation (Variables|Default|GetStartLocation))
  (bind _asbp_mage_base (Utilities|Casting|CastToBP_MageBase _spellowner))
  (bind _fpcamlocation (Variables|/Game/MageGame/MageCharacter/BP_MageBase.BP_MageBase_C|GetFPCamLocation _asbp_mage_base))
  (bind _fpcamforward (Variables|/Game/MageGame/MageCharacter/BP_MageBase.BP_MageBase_C|GetFPCamForward _asbp_mage_base))
  (bind _returnvalue (* _fpcamforward 1e+03))
  (bind _returnvalue_2 (+ _fpcamlocation _returnvalue))
  (bind _returnvalue_3 (Math|Rotator|FindLookatRotation _startlocation _returnvalue_2))
  (|CallParentFunction DeltaSeconds)
  (Utilities|FlowControl|Sequence
    (:then_1
      (Utilities|FlowControl|Gate true
        (:Exit
          (bind (_outhit _returnvalue_4) (Collision|LineTraceByChannel _fpcamlocation _returnvalue_2 "TraceTypeQuery1" false (Utilities|Array|MakeArray self _spellowner) "None"))
          (CallFunction|UpdateSpawnLocation)
          (Utilities|FlowControl|Sequence
            (:then_0
              (CallFunction|Release))
            (:then_1
              (Utilities|FlowControl|Delay 0.1)
              (if _returnvalue_4
                (Variables|Default|SetShootTo (Math|Transform|MakeTransform _startlocation _returnvalue_3))
                (else
                  (Variables|Default|SetShootTo (Math|Transform|MakeTransform _startlocation _returnvalue_3))))
              (bind _returnvalue_5 (Game|SpawnActorfromClass "/Game/MageGame/MageCharacter/Spells/Fire/FlameThrower/BP_Flame_Projectile.BP_Flame_Projectile_C" (Variables|Default|GetShootTo) "Undefined" 0 (Variables|Default|GetSpellOwner) 0.4 1e+01 0))
              (Variables|Default|SetProjectileRef _returnvalue_5)
              (CallFunction|UpdateFlames (Variables|Default|GetShootTo))
              (for _array_element (Variables|Default|GetIgnoredComponents)
                (Collision|IgnoreActorwhenMoving _array_element _returnvalue_5 true)))))))))

(fn ConstructionScript
  (|CallParentFunction))

(fn UpdateSpawnLocation
  (Variables|Default|SetStartLocation (Variables|/Game/MageGame/MageCharacter/BP_MageBase.BP_MageBase_C|Get2HSpawnLocation (.AsBP%20Mage%20Base (Utilities|Casting|CastToBP_MageBase (Variables|Default|GetSpellOwner))))))